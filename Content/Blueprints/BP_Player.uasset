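; Player character that moves with Enhanced Input, interacts with objects and fires popcorn-limited bullets, with HP set up on BeginPlay.
; Movement follows control rotation, and look input updates that rotation with clamped pitch.
; Interact line-traces along the actor's forward vector and calls BPI_Interact on the hit actor; Tick repeats the trace, showing a debug line.
; Shooting decrements PopcornNum and spawns BP_PlayerBullet in front; the scrapped jump graph never runs.
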(event Input|EnhancedActionEvents|EnhancedInputActionIA_Interact
  (params (ActionValue :type Boolean) (ElapsedSeconds :type Float%20%28double-precision%29) (TriggeredSeconds :type Float%20%28double-precision%29) (InputAction :type Input%20Action%20Object%20Reference :default "/Game/Inputs/IA_Interact.IA_Interact"))
  (bind (_outhit _returnvalue) (CallFunction|Trace 2e+02))
  (if _returnvalue
    (bind _asbpi_interact (Utilities|Casting|CastToBPI_Interact (.HitActor (Collision|BreakHitResult _outhit))))
    (Default|Interact _asbpi_interact self)))

(event Input|EnhancedActionEvents|EnhancedInputActionIA_Move
  (params (ActionValue :type Vector%202D%20Structure) (ElapsedSeconds :type Float%20%28double-precision%29) (TriggeredSeconds :type Float%20%28double-precision%29) (InputAction :type Input%20Action%20Object%20Reference :default "/Game/Inputs/IA_Move.IA_Move"))
  (CallFunction|Move (.x ActionValue) (.y ActionValue)))

(event Input|EnhancedActionEvents|EnhancedInputActionIA_Look
  (params (ActionValue :type Vector%202D%20Structure) (ElapsedSeconds :type Float%20%28double-precision%29) (TriggeredSeconds :type Float%20%28double-precision%29) (InputAction :type Input%20Action%20Object%20Reference :default "/Game/Inputs/IA_Look.IA_Look"))
  (CallFunction|UpdateCameraLookRotation (.x ActionValue) (.y ActionValue)))

(event Input|EnhancedActionEvents|EnhancedInputActionIA_Shot
  (params (ActionValue :type Boolean) (ElapsedSeconds :type Float%20%28double-precision%29) (TriggeredSeconds :type Float%20%28double-precision%29) (InputAction :type Input%20Action%20Object%20Reference :default "/Game/Inputs/IA_Shot.IA_Shot"))
  (CallFunction|ActionBullet))

(event EventBeginPlay
  (bind _returnvalue (Pawn|GetController))
  (bind _returnvalue_2 (Pawn|GetControlRotation :!class /Script/Engine.Pawn))
  (bind _asプレイヤーコントローラー (Utilities|Casting|CastToPlayerController _returnvalue))
  (Input|AddMappingContext (PlayerController|LocalPlayerSubsystems|GetEnhancedInputLocalPlayerSubsystem _asプレイヤーコントローラー) "/Game/Inputs/IMC_Default.IMC_Default" 0 "(bIgnoreAllPressedKeysUntilRelease=True,bForceImmediately=False,bNotifyUserSettings=False)")
  (Pawn|SetControlRotation _returnvalue (Math|Rotator|MakeRotator (.roll _returnvalue_2) 3.4e+02 (.yaw _returnvalue_2)))
  (Default|SetHpMax (Variables|Default|GetBP_HpComponent) 10))

(event Collision|EventActorBeginOverlap
  (params (OtherActor :type Actor%20Object%20Reference)))

(event EventTick
  (params (DeltaSeconds :type Float%20%28single-precision%29))
  (CallFunction|Trace 2e+02))

(fn ConstructionScript)

(fn Move
  (params (ScaleValue :type Float%20%28single-precision%29) (ScaleValue2 :type Float%20%28single-precision%29))
  (bind _returnvalue (Pawn|GetControlRotation :!class /Script/Engine.Pawn))
  (Pawn|Input|AddMovementInput (Math|Vector|GetForwardVector _returnvalue) ScaleValue false)
  (Pawn|Input|AddMovementInput (Math|Vector|GetRightVector _returnvalue) ScaleValue2 false))

(fn ActionBullet
  (bind _self self)
  (bind _popcornnum (Variables|Default|GetpopcornNum))
  (if (not (== _popcornnum 0))
    (Math|Integer|DecrementInt _popcornnum
      (:%20%20
        (bind _returnvalue (CallFunction|GetPlayerFrontPosition 1e+02 _self))
        (bind _returnvalue_2 (Game|SpawnActorfromClass "/Game/Blueprints/BP_PlayerBullet.BP_PlayerBullet_C" _returnvalue "Undefined" "MultiplyWithRoot" _self 0))
        (Collision|IgnoreActorwhenMoving (Variables|Character|GetMesh) _returnvalue_2 false)))))

(fn UpdateCameraLookRotation
  (params (x :type Float%20%28double-precision%29) (y :type Float%20%28double-precision%29))
  (bind _returnvalue (Pawn|GetControlRotation :!class /Script/Engine.Pawn))
  (Pawn|SetControlRotation (Game|GetPlayerController 0) (Math|Rotator|MakeRotator (.roll _returnvalue) (Math|Float|Clamp(Float) (+ y (.pitch _returnvalue)) 2.7e+02 3.5e+02) (+ x (.yaw _returnvalue)))))

(fn Trace
  (params (length :type Float%20%28double-precision%29))
  (bind _returnvalue (Transformation|GetActorTransform))
  (bind (_outhit _returnvalue_2) (Collision|LineTraceByChannel (.location _returnvalue) (+ (.location _returnvalue) (* (Math|Vector|GetForwardVector (.rotation _returnvalue)) length)) "TraceTypeQuery3" false 0 "ForOneFrame"))
  (return _outhit _returnvalue_2))