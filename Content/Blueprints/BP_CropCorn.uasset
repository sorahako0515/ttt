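; BP_CropCorn is a corn crop actor that grows on a timer, is harvested by the player, and can be destroyed.
; When the timer fires, it shows the corn mesh; an overlapping BP_Player harvests it immediately or on later overlap, gaining corn, reverting it to a sprout and restarting the timer.
; An HP component with a custom-colored bar triggers death, which disables collision and animates vertical scale on a timeline before destroying the actor.
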(event Custom|OnDeath_イベント
  (|Death))

(event Custom|OnGrown
  (bind _overlappingactors (Collision|GetOverlappingActors "/Game/Blueprints/BP_Player.BP_Player_C" :!class /Script/Engine.Actor))
  (CallFunction|UpdateCropState "NewEnumerator0")
  (if (== (Utilities|Array|Length _overlappingactors) 1)
    (bind _asbp_player (Utilities|Casting|CastToBP_Player (Utilities|Array|Get(acopy) _overlappingactors)))
    (CallFunction|Harvest _asbp_player)
    (Utilities|Time|SetTimerbyEvent (delegate Custom|OnGrown) (Variables|Default|Getinterval))))

(event EventBeginPlay
  (CallFunction|Setup)
  (EventDispatchers|AssignOnDeath (Variables|Default|GetBP_HpComponent) (delegate Custom|OnDeath_イベント))
  (Utilities|Time|SetTimerbyEvent (delegate Custom|OnGrown) (Variables|Default|Getinterval)))

(event Collision|EventActorBeginOverlap
  (params (OtherActor :type Actor%20Object%20Reference))
  (bind _asbp_player (Utilities|Casting|CastToBP_Player OtherActor))
  (if (Utilities|Enum|Equal(Enum) (Variables|Default|GetcropState) "NewEnumerator0")
    (CallFunction|Harvest _asbp_player)
    (Utilities|Time|SetTimerbyEvent (delegate Custom|OnGrown) (Variables|Default|Getinterval))))

(fn ConstructionScript)

(fn UpdateCropState
  (params (cropState :type E_CropState%20Enum :default "NewEnumerator1"))
  (if (Utilities|Enum|NotEqual(Enum) cropState (Variables|Default|GetcropState))
    (bind _output_get (Variables|Default|SetcropState cropState))
    (Rendering|SetVisibility (Variables|Default|GetMesh_Sprout) (Utilities|Enum|Equal(Enum) _output_get "NewEnumerator1") false)
    (Rendering|SetVisibility (Variables|Default|GetMesh_Corn) (Utilities|Enum|Equal(Enum) _output_get "NewEnumerator0") false)))

(fn Setup
  (bind _bpui_hp (Variables|Default|GetBPUI_HP))
  (Default|SetHpMax (Variables|Default|GetBP_HpComponent) (Variables|Default|GethpMax))
  (Variables|/Game/Blueprints/BPUI_HP.BPUI_HP_C|SetisHpMaxVisible _bpui_hp false)
  (Variables|/Game/UI/UI_HpBar.UI_HpBar_C|SetbarColor (Variables|/Game/Blueprints/BPUI_HP.BPUI_HP_C|GetuiHpBar _bpui_hp) "(R=0.776042,G=0.656844,B=0.058770,A=1.000000)")
  (Default|UpdateHpBar _bpui_hp)
  (return))

(fn Harvest
  (params (player :type BP%20Player%20Object%20Reference))
  (Math|Integer|IncrementInt (Variables|/Game/Blueprints/BP_Player.BP_Player_C|GetcornNum player)
    (:%20%20
      (CallFunction|UpdateCropState "NewEnumerator1"))))