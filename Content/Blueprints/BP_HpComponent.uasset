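; BP_HpComponent tracks current and maximum HP for its owner and announces health changes and death.
; SetHpMax sets the maximum and refills HP, while AddHp applies a delta clamped between zero and max, ignoring calls once dead.
; AddHp fires OnHpChanged with the requested delta and instigator, then OnDeath upon reaching zero, with debug prints.
; Helper functions report death, full HP and the HP ratio.
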(event EventBeginPlay)

(event EventTick
  (params (DeltaSeconds :type Float%20%28single-precision%29)))

(fn SetHpMax
  (params (hpMax :type Integer))
  (bind _output_get (Variables|Default|SethpMax hpMax))
  (Variables|Default|Sethp _output_get))

(fn AddHp
  (params (AddHp :type Integer) (Instigator :type Actor%20Object%20Reference))
  (Development|PrintString (Utilities|String|Append "NowHp:" (Utilities|String|ToString(Integer) (Variables|Default|Gethp)) "damagedHp:" (Utilities|String|ToString(Integer) AddHp)))
  (bind _isdead (CallFunction|IsDead))
  (if (not _isdead)
    (Variables|Default|Sethp (Math|Integer|Clamp(Integer) (+ AddHp (Variables|Default|Gethp)) 0 (Variables|Default|GethpMax)))
    (Default|CallOnHpChanged AddHp Instigator)
    (bind _isdead_2 (CallFunction|IsDead))
    (if _isdead_2
      (Development|PrintString "OnDeath" true true "(R=1.000000,G=0.101989,B=0.161720,A=1.000000)")
      (Default|CallOnDeath))))

(fn IsDead
  (return (== (Variables|Default|Gethp) 0)))

(fn IsHpFull
  (return (== (Variables|Default|GethpMax) (Variables|Default|Gethp))))

(fn CalcHpPercent
  (return (/ (Math|Conversions|ToFloat(Integer) (Variables|Default|Gethp)) (Math|Conversions|ToFloat(Integer) (Variables|Default|GethpMax)))))