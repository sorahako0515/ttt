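; BP_PopcornMachineManager manages a list of popcorn machines and activates another one on request.
; GetEmptyMachine returns the index of the first hidden machine in MachineList.
; AddPopcornMachine checks that result against -1, then calls SetActivate on the entry indexed by the comparison converted to an integer, not the found index.
; Event graph and construction script are empty.
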(event EventBeginPlay)

(event Collision|EventActorBeginOverlap
  (params (OtherActor :type Actor%20Object%20Reference)))

(event EventTick
  (params (DeltaSeconds :type Float%20%28single-precision%29)))

(fn ConstructionScript)

(fn GetEmptyMachine
  (bind (_array_element _array_index) (Utilities|Array|ForEachLoopwithBreak (Variables|Default|GetmachineList) :!label _label)
    (:LoopBody
      (if (Variables|/Script/Engine.Actor|GetbHidden _array_element)
        (LocalVariables|Setret _array_index)
        (goto _label Break)))
    (:Completed
      (return (LocalVariables|Getret)))))

(fn AddPopcornMachine
  (bind _emptymachine (CallFunction|GetEmptyMachine))
  (if (!= _emptymachine -1)
    (Default|SetActivate (Utilities|Array|Get(acopy) (Variables|Default|GetmachineList) (Math|Conversions|ToInteger(Boolean) (!= _emptymachine -1))) true)))