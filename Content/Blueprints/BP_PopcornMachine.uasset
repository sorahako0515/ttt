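; BP_PopcornMachine is a machine that turns a player's corn into popcorn.
; Interaction or player overlap starts making when Idle and corn is available, or hands over finished popcorn, then immediately tries another batch.
; A re-armed timer advances the widget's progress bar until done, with popcorn yield read from BP_GameMode.
; An enable flag toggles visibility and box collision, and the widget billboards every tick.
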(event Custom|OnMaking
  (bind _ui (Variables|Default|GetUI))
  (bind _interval (Variables|Default|Getinterval))
  (bind _bar (Variables|/Game/UI/UI_Machine.UI_Machine_C|GetBar _ui))
  (bind _output_get (Variables|Default|Settimer (+ (Variables|Default|Gettimer) (Variables|Default|Getduration))))
  (Progress|SetPercent _bar (/ _output_get _interval))
  (if (>= _output_get _interval)
    (Progress|SetPercent _bar 0.0)
    (CallFunction|SetState "NewEnumerator2")
    (else
      (Utilities|Time|SetTimerbyEvent (delegate Custom|OnMaking) (Variables|Default|Getduration)))))

(event EventBeginPlay
  (CallFunction|SetActivate (Variables|Default|GetisEnable))
  (bind _asui_machine (Utilities|Casting|CastToUI_Machine (UserInterface|GetUserWidgetObject (Variables|Default|GetWidget))))
  (bind _output_get (Variables|Default|SetUI _asui_machine))
  (Default|SetState _output_get "NewEnumerator0"))

(event Collision|EventActorBeginOverlap
  (params (OtherActor :type Actor%20Object%20Reference))
  (bind _asbp_player (Utilities|Casting|CastToBP_Player OtherActor))
  (if true
    (CallFunction|DoInteract _asbp_player)))

(event EventTick
  (params (DeltaSeconds :type Float%20%28single-precision%29))
  (CallFunction|SetBillboardPosition (Variables|Default|GetWidget)))

(event EventInteract
  (params (player :type BP%20Player%20Object%20Reference))
  (CallFunction|DoInteract player))

(fn ConstructionScript)

(fn SetState
  (params (state :type E_PopconeMachineState%20Enum :default "NewEnumerator0"))
  (if (Utilities|Enum|NotEqual(Enum) state (Variables|Default|Getstate))
    (bind _output_get (Variables|Default|Setstate state))
    (Default|SetState (Variables|Default|GetUI) _output_get)
    (switch Utilities|FlowControl|Switch|SwitchonE_PopconeMachineState _output_get
      (:NewEnumerator1
        (Variables|Default|Settimer 0.0)
        (Utilities|Time|SetTimerbyFunctionName 0 "OnMaking" (Variables|Default|Getduration))))))

(fn DoInteract
  (params (player :type BP%20Player%20Object%20Reference))
  (switch Utilities|FlowControl|Switch|SwitchonE_PopconeMachineState (Variables|Default|Getstate) :!label _label
    (:NewEnumerator0
      (if (> (Variables|/Game/Blueprints/BP_Player.BP_Player_C|GetcornNum player) 0)
        (Default|AddCorn player -1)
        (CallFunction|SetState "NewEnumerator1")))
    (:NewEnumerator2
      (bind _popcornmakenum (|GetPopcornMakeNum))
      (Default|AddPopcorn player _popcornmakenum)
      (CallFunction|SetState "NewEnumerator0")
      (goto _label))))

(fn SetActivate
  (params (enable :type Boolean))
  (Rendering|SetActorHiddenInGame self (not enable))
  (bind _output_get (Variables|Default|SetisEnable enable))
  (Collision|SetCollisionEnabled (Variables|Default|GetBox) (select _output_get "QueryAndPhysics" "NoCollision")))