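; Manager for a grid of crop soil, forwarding planting requests by X/Y to the BP_Soil entries in SoilList.
; BeginPlay plants two starting crops in the first soil entry.
; PutCropRandom plants at a random point from GetRandomEmptySoil, which scans each soil's Crops array.
; Despite its name, that scan collects slots whose crop IsValid, and OnCropDead is an empty stub.
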(event EventBeginPlay
  (CallFunction|PutCrop 3)
  (CallFunction|PutCrop 5))

(event Collision|EventActorBeginOverlap
  (params (OtherActor :type Actor%20Object%20Reference)))

(event EventTick
  (params (DeltaSeconds :type Float%20%28single-precision%29)))

(fn ConstructionScript)

(fn PutCrop
  (params (x :type Integer) (y :type Integer))
  (if (>= x 0)
    (Default|PutCrop (Utilities|Array|Get(acopy) (Variables|Default|GetsoilList) y) x)))

(fn OnCropDead)

(fn GetRandomEmptySoil
  (bind _emptypositions (LocalVariables|GetemptyPositions))
  (bind _returnvalue (Utilities|Array|IsNotEmpty _emptypositions))
  (for (_array_element _array_index) (Variables|Default|GetsoilList)
    (bind _asbp_soil (Utilities|Casting|CastToBP_Soil _array_element))
    (for (_array_element_2 _array_index_2) (Variables|/Game/Blueprints/BP_Soil.BP_Soil_C|Getcrops _asbp_soil)
      (Utilities|IsValid _array_element_2
        (:Is%20Valid
          (Utilities|Array|Add _emptypositions (Utilities|Struct|MakeIntPoint _array_index_2 _array_index))))))
  (if _returnvalue
    (bind _output_get (LocalVariables|SetreturnPoint (.OutItem (Utilities|Array|Random _emptypositions)))))
  (return _returnvalue _output_get))

(fn PutCropRandom
  (bind (_hasemptyslot _emptyposition) (CallFunction|GetRandomEmptySoil))
  (if _hasemptyslot
    (CallFunction|PutCrop (.x _emptyposition) (.y _emptyposition))))