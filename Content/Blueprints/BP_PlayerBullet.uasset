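; BP_PlayerBullet is the player's bullet actor, which damages whatever it hits that has health.
; On BeginPlay it snaps its Z position to a fixed height, keeping X, Y, rotation and scale.
; On overlap with an actor that has a BP_HpComponent, it applies negated Damage through AddHp as instigator, then destroys itself.
; Other overlaps are ignored, and the graph contains no movement logic.
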(event EventBeginPlay
  (bind _returnvalue (Transformation|GetActorTransform))
  (bind (_location _rotation _scale) (Math|Transform|BreakTransform _returnvalue))
  (Transformation|SetActorTransform (Math|Transform|MakeTransform (Math|Vector|MakeVector (.x _location) (.y _location) 2e+01) _rotation _scale)))

(event Collision|EventActorBeginOverlap
  (params (OtherActor :type Actor%20Object%20Reference))
  (bind _returnvalue (Actor|GetComponentbyClass OtherActor "/Game/Blueprints/BP_HpComponent.BP_HpComponent_C"))
  (Utilities|IsValid _returnvalue
    (:Is%20Valid
      (Default|AddHp _returnvalue (* (Variables|Default|Getdamage) -1) self)
      (Actor|DestroyActor))))

(event EventTick
  (params (DeltaSeconds :type Float%20%28single-precision%29)))

(fn ConstructionScript)