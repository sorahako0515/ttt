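; BP_Shop is an in-world shop that opens the shop UI through BP_HUD when BP_Player overlaps it, passing its ShopItems and itself as receiver.
; On ChangeState it refreshes a shop button with the item name plus corn and popcorn prices.
; Each buy button is enabled only if the player holds enough of that currency.
; The Buy event only prints a debug string.
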(event EventBeginPlay)

(event Collision|EventActorBeginOverlap
  (params (OtherActor :type Actor%20Object%20Reference))
  (bind _asbp_player (Utilities|Casting|CastToBP_Player OtherActor))
  (if true
    (CallFunction|DoInteract _asbp_player)))

(event EventTick
  (params (DeltaSeconds :type Float%20%28single-precision%29)))

(event EventBuy
  (params (shopItem :type F%20Shop%20Item%20Structure) (asCorn :type Boolean))
  (Development|PrintString "onBuy"))

(event EventChangeState
  (params (shopButton :type UIP%20Shop%20Button%20Object%20Reference))
  (CallFunction|OnChangeState shopButton))

(fn ConstructionScript)

(fn DoInteract
  (params (player :type BP%20Player%20Object%20Reference))
  (bind _asbp_hud (Utilities|Casting|CastToBP_HUD (HUD|GetHUD (Game|GetPlayerController 0))))
  (Default|ShowShopUI _asbp_hud (Variables|Default|GetShop%20Items) self))

(fn OnChangeState
  (params (shopButton :type UIP%20Shop%20Button%20Object%20Reference))
  (bind _shopitem (Variables|/Game/UI/UIP_ShopButton.UIP_ShopButton_C|GetshopItem shopButton))
  (|SetItemName shopButton (.name _shopitem))
  (bind _asbp_player (|getPlayer))
  (|SetCorn _asbp_player shopButton (.cornprice _shopitem))
  (|SetPopcorn _asbp_player shopButton (.popcornprice _shopitem)))