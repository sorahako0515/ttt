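; BPUI_HP is a widget component that shows its owner's HP as a world-space bar.
; On BeginPlay it finds the owner's BP_HpComponent and UI_HpBar widget and disables shadow casting, or prints an error and destroys itself if setup fails.
; HP change events update the bar's percent, hiding it at full HP unless IsHpMaxVisible is set.
; Each Tick calls SetBillboardPosition to billboard the component.
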(event Custom|OnHpChanged_イベント
  (params (addHp :type Integer) (Instigator :type Actor%20Object%20Reference))
  (CallFunction|UpdateHpBar))

(event EventBeginPlay
  (Class|WidgetComponent|SetWidgetSpace "World")
  (bind _result (CallFunction|Setup))
  (if _result
    (EventDispatchers|AssignOnHpChanged (Variables|Default|GethpComponent) (delegate Custom|OnHpChanged_イベント))
    (else
      (Development|PrintString "Not Find Hp Component" true true "(R=0.963542,G=0.129936,B=0.158695,A=1.000000)")
      (Components|DestroyComponent))))

(event EventTick
  (params (DeltaSeconds :type Float%20%28single-precision%29))
  (CallFunction|SetBillboardPosition self))

(fn Setup
  (LocalVariables|Setret false)
  (bind _output_get (Variables|Default|SethpComponent (Actor|GetComponentbyClass (Components|GetOwner) "/Game/Blueprints/BP_HpComponent.BP_HpComponent_C")))
  (Utilities|IsValid _output_get
    (:Is%20Valid
      (Variables|Default|SethpComponent _output_get)
      (bind _asui_hp_bar (Utilities|Casting|CastToUI_HpBar (UserInterface|GetUserWidgetObject))
        (:then
          (Variables|Default|SetuiHpBar _asui_hp_bar)
          (Rendering|SetCastShadow false) ; UIの影無効化
          (LocalVariables|Setret true))
        (:CastFailed
          _)))
    (:Is%20Not%20Valid
      _))
  (return (LocalVariables|Getret)))

(fn UpdateHpBar
  (bind _hpcomponent (Variables|Default|GethpComponent))
  (bind _uihpbar (Variables|Default|GetuiHpBar))
  (bind _percent (Default|CalcHpPercent _hpcomponent))
  (Default|SetPercent _uihpbar _percent)
  (if (not (Variables|Default|GetisHpMaxVisible))
    (bind _ishpfull (Default|IsHpFull _hpcomponent))
    (Variables|/Game/UI/UI_HpBar.UI_HpBar_C|SetisBarVisible _uihpbar (select _ishpfull "Hidden" "Visible"))))