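; Enemy rat character that attacks BP_CropCorn crops, falling back to the player when none exist.
; SearchTarget picks the nearest crop, AIMoveTo approaches it, then a delayed loop damages its BP_HpComponent, retargeting on failure or target death.
; GetAttackTarget toggles attack collision, but its overlap check does not affect the result.
; On its own death, it increments the GameMode kill score and plays a timeline squash before destroying itself.
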(event Custom|OnDeath_イベント
  (params (own :type BP%20Hp%20Component%20Object%20Reference))
  (bind _rat1 (Variables|Default|GetRat1))
  (|AddRatKillScore
    (:%20%20
      (Class|NavMovementComponent|StopActiveMovement (Variables|Character|GetCharacterMovement))
      (Collision|SetCollisionEnabled _rat1 "NoCollision")
      (|RatDeadAnimation _rat1))))

(event Custom|OnTargetDead
  (params (own :type BP%20Hp%20Component%20Object%20Reference))
  (bind _target (Variables|Default|Gettarget))
  (CallFunction|SearchTarget :!label _label)
  (EventDispatchers|BindEventtoOnDeath (Actor|GetComponentbyClass _target "/Game/Blueprints/BP_HpComponent.BP_HpComponent_C") (delegate Custom|OnTargetDead))
  (AI|AIMoveTo self "0, 0, 0" _target 5.0 false
    (:OnSuccess
      (bind _targethpcomponent (CallFunction|GetAttackTarget :!label _label_2))
      (Utilities|IsValid _targethpcomponent
        (:Is%20Valid
          (Default|AddHp _targethpcomponent -1 self)
          (Utilities|FlowControl|Delay 2.0)
          (goto _label_2))
        (:Is%20Not%20Valid
          (Development|PrintString "not Damaged")
          (goto _label))))
    (:OnFail
      (goto _label))))

(event EventBeginPlay
  (bind _target (Variables|Default|Gettarget))
  (bind _bp_hpcomponent (Variables|Default|GetBP_HpComponent))
  (Default|SetHpMax _bp_hpcomponent (Variables|Default|GethpMax))
  (Default|UpdateHpBar (Variables|Default|GetBPUI_HP))
  (EventDispatchers|AssignOnDeath _bp_hpcomponent (delegate Custom|OnDeath_イベント))
  (CallFunction|SearchTarget :!label _label)
  (EventDispatchers|BindEventtoOnDeath (Actor|GetComponentbyClass _target "/Game/Blueprints/BP_HpComponent.BP_HpComponent_C") (delegate Custom|OnTargetDead))
  (AI|AIMoveTo self "0, 0, 0" _target 5.0 false
    (:OnSuccess
      (bind _targethpcomponent (CallFunction|GetAttackTarget :!label _label_2))
      (Utilities|IsValid _targethpcomponent
        (:Is%20Valid
          (Default|AddHp _targethpcomponent -1 self)
          (Utilities|FlowControl|Delay 2.0)
          (goto _label_2))
        (:Is%20Not%20Valid
          (Development|PrintString "not Damaged")
          (goto _label))))
    (:OnFail
      (goto _label))))

(event Collision|EventActorBeginOverlap
  (params (OtherActor :type Actor%20Object%20Reference)))

(event EventTick
  (params (DeltaSeconds :type Float%20%28single-precision%29)))

(fn ConstructionScript)

(fn SearchTarget
  (bind _outactors (Actor|GetAllActorsOfClass "/Game/Blueprints/BP_CropCorn.BP_CropCorn_C"))
  (if (Utilities|Array|IsNotEmpty _outactors)
    (for _array_element _outactors
      (if (or (< (Math|Vector|Distance(Vector) (Transformation|GetActorLocation _array_element) (Transformation|GetActorLocation)) (LocalVariables|Getdistance)) (< (LocalVariables|Getdistance) 0.0))
        (Variables|Default|Settarget _array_element)
        (LocalVariables|Setdistance (Math|Vector|Distance(Vector) (Transformation|GetActorLocation _array_element) (Transformation|GetActorLocation)))))
    (else
      (Variables|Default|Settarget (Game|Player|GetPlayerPawn 0)))))

(fn GetAttackTarget
  (bind _collisionattack (Variables|Default|GetcollisionAttack))
  (bind _target (Variables|Default|Gettarget))
  (Utilities|IsValid _target
    (:Is%20Valid
      (Collision|SetCollisionEnabled _collisionattack "QueryAndPhysics")
      (if (!= (Utilities|Array|FindItem (Collision|GetOverlappingActors "/Game/Blueprints/BP_CropCorn.BP_CropCorn_C" :!class /Script/Engine.Actor) _target) -1)
        _
        (else
          _))
      (LocalVariables|SetretTargetHpComponent (Actor|GetComponentbyClass _target "/Game/Blueprints/BP_HpComponent.BP_HpComponent_C"))
      (Collision|SetCollisionEnabled _collisionattack "NoCollision"))
    (:Is%20Not%20Valid
      _))
  (return (LocalVariables|GetretTargetHpComponent)))