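; Enemy spawner actor that spawns a BP_EnemyRat1 whenever its Tick-accumulated timer reaches SpawnInterval.
; CalcSpawnPosition scatters spawns around the world origin at fixed height, rolling radius and angle separately for X and Y, so points don't form a true ring.
; Yaw comes from 画面中央に向く回転計算 (face screen center), whose look-at calculation toward the spawner, with an offset, appears unconnected.
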(event EventBeginPlay)

(event Collision|EventActorBeginOverlap
  (params (OtherActor :type Actor%20Object%20Reference)))

(event EventTick
  (params (DeltaSeconds :type Float%20%28single-precision%29))
  (bind _output_get (Variables|Default|SetspawnCount (+ DeltaSeconds (Variables|Default|GetspawnCount))))
  (if (>= _output_get (Variables|Default|GetspawnInterval))
    (Variables|Default|SetspawnCount 0.0)
    (bind _position (CallFunction|CalcSpawnPosition))
    (Game|SpawnActorfromClass "/Game/Blueprints/BP_EnemyRat1.BP_EnemyRat1_C" (Math|Transform|MakeTransform _position (Math|Rotator|MakeRotator 0.0 0.0 (|画面中央に向く回転計算 _position))) "Undefined" "MultiplyWithRoot" 0 0)))

(fn ConstructionScript)

(fn CalcSpawnPosition
  (bind _returnvalue (Math|Random|RandomFloatinRange 0.0 3.6e+02))
  (bind _radiusmax (Variables|Default|GetradiusMax))
  (bind _radiusmin (Variables|Default|GetradiusMin))
  (bind _returnvalue_2 (Math|Random|RandomFloatinRange _radiusmin _radiusmax))
  (return (Math|Vector|MakeVector (* _returnvalue_2 (Math|Trig|Cos(Radians) _returnvalue)) (* _returnvalue_2 (Math|Trig|Sin(Radians) _returnvalue)) 5e+01)))